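; Enemy character that chases the first GasolineCircleCharacter, re-finding it and issuing a simple move-to every Tick.
; Incoming damage feeds the Health component, whose change event spawns a randomly offset DisplayDamageActor showing the hit.
; On death it unpossesses, sets a lifespan for cleanup and plays a death montage.
; When the montage completes, it switches the mesh to ragdoll physics, ignores pawns on the capsule and only then sets IsDead.
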(event OnHealthChange(Health)
  (params (Health :type Float%20%28single-precision%29) (Damage :type Float%20%28single-precision%29))
  (if (not (Variables|Default|GetbIsDead))
    (bind _returnvalue (Game|SpawnActorfromClass "/Game/Environment/Blueprint/DisplayDamageActor.DisplayDamageActor_C" (Math|Transform|MakeTransform (+ (+ (Math|Vector|MakeVector (Math|Random|RandomFloatinRange -1e+01 1e+01) (Math|Random|RandomFloatinRange -1e+01 1e+01) 0.0) (Variables|Default|GetSpawnOffsetActorLocation)) (Transformation|GetActorLocation))) "AlwaysSpawn" 0 0))
    (Default|InitActor _returnvalue Damage Health)))

(event OnDead(Health)
  (bind _mesh (Variables|Character|GetMesh))
  (if (not (Variables|Default|GetbIsDead))
    (CallFunction|DeadEvent)
    (Animation|Montage|PlayMontage _mesh "/Game/Blueprints/Character/Enemy/Anim/EnemyDeath_Montage.EnemyDeath_Montage"
      (:OnCompleted
        (Collision|SetCollisionEnabled _mesh "PhysicsOnly")
        (Collision|SetCollisionResponsetoChannel (Variables|Collision|GetCapsuleComponent) "ECC_Pawn" "ECR_Ignore")
        (Collision|SetCollisionProfileName _mesh "PhysicsActor" true :!class /Script/Engine.PrimitiveComponent)
        (Physics|SetSimulatePhysics _mesh true)
        (Variables|Default|SetbIsDead true)))))

(event EventTick
  (params (DeltaSeconds :type Float%20%28single-precision%29))
  ;[1 1 1] Bullting character logic
  (bind _outactors (Actor|GetAllActorsOfClass "/Script/GasolineCircle.GasolineCircleCharacter"))
  (Utilities|IsValid (Utilities|Array|Get(acopy) _outactors)
    (:Is%20Valid
      (AI|Navigation|SimpleMovetoActor (Pawn|GetController) (Utilities|Array|Get(acopy) _outactors)))))

(event Game|Damage|EventAnyDamage
  (params (Damage :type Float%20%28single-precision%29) (DamageType :type Damage%20Type%20Object%20Reference) (InstigatedBy :type Controller%20Object%20Reference) (DamageCauser :type Actor%20Object%20Reference))
  (if (not (Variables|Default|GetbIsDead))
    (Class|HealthComponent|ChangeCurrentHealth (Variables|Default|GetHealth) (* Damage -1.0))))

(fn ConstructionScript)

(fn DeadEvent
  (Pawn|UnPossess (Pawn|GetController))
  (Actor|SetLifeSpan 2e+01))