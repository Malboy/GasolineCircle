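; BP_CanDamageActor is a damageable environment actor that shows damage feedback and is destroyed when its health runs out.
; Any damage received is passed as a negative change to its Health component.
; Each health change spawns a DisplayDamageActor at an unrotated offset from the actor's location, with slight random XY jitter, and initializes it with damage and current health.
; The Health component's death event destroys the actor.
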(event OnHealthChange(Health)
  (params (Health :type Float%20%28single-precision%29) (Damage :type Float%20%28single-precision%29))
  (bind _returnvalue (Game|SpawnActorfromClass "/Game/Environment/Blueprint/DisplayDamageActor.DisplayDamageActor_C" (Math|Transform|MakeTransform (+ (+ (Math|Vector|MakeVector (Math|Random|RandomFloatinRange -1e+01 1e+01) (Math|Random|RandomFloatinRange -1e+01 1e+01) 0.0) (Variables|Default|GetLocalPointSpawnHealthNumber)) (Transformation|GetActorLocation))) "AlwaysSpawn" 0 0))
  (Default|InitActor _returnvalue Damage Health))

(event OnDead(Health)
  (Actor|DestroyActor))

(event EventBeginPlay)

(event Game|Damage|EventAnyDamage
  (params (Damage :type Float%20%28single-precision%29) (DamageType :type Damage%20Type%20Object%20Reference) (InstigatedBy :type Controller%20Object%20Reference) (DamageCauser :type Actor%20Object%20Reference))
  (Class|HealthComponent|ChangeCurrentHealth (Variables|Default|GetHealth) (* Damage -1.0)))

(fn ConstructionScript)